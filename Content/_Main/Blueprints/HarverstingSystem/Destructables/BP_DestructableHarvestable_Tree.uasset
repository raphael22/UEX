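; BP_DestructableHarvestable_Tree is a tree piece in the harvesting system's destructables that gets pushed when it spawns and removes itself afterward.
; On BeginPlay it applies an acceleration-based force to its Capsule along a Direction scaled by Force, then destroys itself after a ten-second delay.
; The authority switch leads nowhere on either branch, and the construction script only calls the parent's.
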(event EventBeginPlay
  (Networking|SwitchHasAuthority
    (:Authority
      _)
    (:Remote
      _))
  (CallFunction|AddForce)
  (Utilities|FlowControl|Delay 1e+01)
  (Actor|DestroyActor))

(fn ConstructionScript
  (|CallParentFunction))

(fn AddForce
  (Physics|AddForce (Variables|Default|GetCapsule) (* (Variables|Default|GetDirection) (LocalVariables|GetForce)) "None" true))