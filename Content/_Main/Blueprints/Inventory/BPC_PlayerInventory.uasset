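; Player inventory component that extends a parent item container with slot drop handling and UI slot syncing.
; Drops from the player inventory or hotbar are passed to the source container's TransferItem, targeting the dropped index in this component.
; Add and remove overrides run the parent logic, then message the owning character's controller to update or reset the affected slot.
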(event EventBeginPlay
  (|CallParentFunction) ; This node is disabled and will not be called.\nDrag off pins to build functionality.
)

(event EventTick
  (params (DeltaSeconds :type Float%20%28single-precision%29))
  (|CallParentFunction DeltaSeconds) ; This node is disabled and will not be called.\nDrag off pins to build functionality.
)

(fn HandleSlotDrop
  (params (FromContainer :type BPC%20Items%20Container%20Object%20Reference) (FromIndex :type Integer) (DroppedIndex :type Integer))
  (LocalVariables|SetLocalFromContainer FromContainer)
  (LocalVariables|SetLocalFromIndex FromIndex)
  (LocalVariables|SetLocalDroppedIndex DroppedIndex)
  (switch Utilities|FlowControl|Switch|SwitchonE_ContainerType (Variables|/Game/_Main/Blueprints/Inventory/BPC_ItemsContainer.BPC_ItemsContainer_C|GetContainerType (LocalVariables|GetLocalFromContainer))
    (:NewEnumerator0
      _)
    (:NewEnumerator1
      _))
  (Default|TransferItem (LocalVariables|GetLocalFromContainer) self (LocalVariables|GetLocalDroppedIndex) (LocalVariables|GetLocalFromIndex))
  (return))

(fn AddItemtoIndex
  (params (Item :type S%20Item%20Info%20Structure) (LocalSpecificIndex :type Integer) (FromIndex :type Integer))
  (LocalVariables|SetLocalIndex LocalSpecificIndex)
  (bind _success_ (|CallParentFunction Item LocalSpecificIndex FromIndex))
  (bind _controllerref (Class|BPICharacter|GetControllerfromCharacter(Message) (Components|GetOwner)))
  (Default|UpdateItemSlot _controllerref (Variables|Default|GetContainerType) (LocalVariables|GetLocalIndex) (CallFunction|GetItematIndex (LocalVariables|GetLocalIndex)))
  (return _success_))

(fn RemoveItematIndex
  (params (Index :type Integer))
  (LocalVariables|SetLocalIndex Index)
  (bind _success_ (|CallParentFunction Index))
  (bind _controllerref (Class|BPICharacter|GetControllerfromCharacter(Message) (Components|GetOwner)))
  (Default|ResetItemSlot _controllerref (Variables|Default|GetContainerType) (LocalVariables|GetLocalIndex))
  (return _success_))