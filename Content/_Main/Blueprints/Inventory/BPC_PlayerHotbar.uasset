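; Player hotbar component, a child of an item container component, that holds the items in the player's hotbar slots.
; CheckHotbar reports whether a slot is filled and its item type, while HandleSlotDrop transfers items dropped from the player inventory or hotbar.
; Add and remove overrides call the parent, then update or reset the slot through controller interface messages.
; Removal also tells the character to dequip the current item at that index.
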(event EventBeginPlay)

(event EventTick
  (params (DeltaSeconds :type Float%20%28single-precision%29)))

(fn CheckHotbar
  (params (Index :type Integer))
  (bind _items (Variables|Default|GetItems))
  (bind _output (Utilities|Array|Get(acopy) _items Index))
  (bind (_itemid _itemicon _itemname _itemdescription _itemrarity _itemtype) (Utilities|Struct|BreakS_ItemInfo _output))
  (if (== _itemid 0)
    (return false "NewEnumerator0")
    (else
      (return true _itemtype))))

(fn HandleSlotDrop
  (params (FromContainer :type BPC%20Items%20Container%20Object%20Reference) (FromIndex :type Integer) (DroppedIndex :type Integer))
  (LocalVariables|SetLocalDroppedIndex DroppedIndex)
  (LocalVariables|SetLocalFromIndex FromIndex)
  (LocalVariables|SetLocalFromContainer FromContainer)
  (switch Utilities|FlowControl|Switch|SwitchonE_ContainerType (Variables|/Game/_Main/Blueprints/Inventory/BPC_ItemsContainer.BPC_ItemsContainer_C|GetContainerType (LocalVariables|GetLocalFromContainer))
    (:NewEnumerator0
      _)
    (:NewEnumerator1
      _))
  (Default|TransferItem (LocalVariables|GetLocalFromContainer) self (LocalVariables|GetLocalDroppedIndex) (LocalVariables|GetLocalFromIndex))
  (return))

(fn AddItemtoIndex
  (params (Item :type S%20Item%20Info%20Structure) (LocalSpecificIndex :type Integer) (FromIndex :type Integer))
  (LocalVariables|SetLocalIndex LocalSpecificIndex)
  (bind _success_ (|CallParentFunction Item LocalSpecificIndex FromIndex))
  (bind _controllerref (Class|BPICharacter|GetControllerfromCharacter(Message) (Components|GetOwner)))
  (Default|UpdateItemSlot _controllerref (Variables|Default|GetContainerType) (LocalVariables|GetLocalIndex) (CallFunction|GetItematIndex (LocalVariables|GetLocalIndex)))
  (return _success_))

(fn RemoveItematIndex
  (params (Index :type Integer))
  (LocalVariables|SetLocalIndex Index)
  (bind _success_ (|CallParentFunction Index))
  (bind _controllerref (Class|BPICharacter|GetControllerfromCharacter(Message) (Components|GetOwner)))
  (Default|ResetItemSlot _controllerref (Variables|Default|GetContainerType) (LocalVariables|GetLocalIndex))
  (bind _characterref (Class|BPICharacter|GetCharacterRef(Message) (Components|GetOwner)))
  (Default|DequipCurrentItem _characterref (LocalVariables|GetLocalIndex))
  (return _success_))