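; Player controller that owns the client-side main HUD and relays inventory changes to it.
; On BeginPlay the remote side creates W_MainWidget, and Tab or I toggles the inventory along with cursor and input mode.
; Slot update and reset events find the slot widget by container and index, with only inventory and hotbar mapped.
; A further event forwards collected-item popups to the main widget.
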(event Custom|InventoryOnClient
  (bind _self self)
  (bind _mainwidgetref (Variables|Default|GetMainWidgetRef))
  (if (Variables|Default|GetInventoryShown?)
    (Default|SetInventoryVisibility _mainwidgetref false)
    (Variables|Default|SetbShowMouseCursor false)
    (Input|SetInputModeGameOnly _self false)
    (Variables|Default|SetInventoryShown? false)
    (else
      (Default|SetInventoryVisibility _mainwidgetref true)
      (Variables|Default|SetbShowMouseCursor true)
      (Input|SetInputModeGameandUI _self 0 "DoNotLock" true false)
      (Variables|Default|SetInventoryShown? true))))

(event Custom|ShowItemWidget
  (params (ResourceImage :type Texture%202D%20Object%20Reference) (ResourceQuantity :type Integer) (ResourceName :type Text))
  (Default|ShowItemCollected (Variables|Default|GetMainWidgetRef) ResourceImage ResourceQuantity ResourceName))

(event Custom|UpdateItemSlot
  (params (Container :type E_ContainerType%20Enum :default "NewEnumerator0") (Index :type Integer) (ItemInfo :type S%20Item%20Info%20Structure))
  (bind _widget (CallFunction|GetInventoryWidget Container Index))
  (Utilities|IsValid _widget
    (:Is%20Valid
      (Default|UpdateSlot _widget ItemInfo))))

(event Custom|ResetItemSlot
  (params (Container :type E_ContainerType%20Enum :default "NewEnumerator0") (Index :type Integer))
  (bind _widget (CallFunction|GetInventoryWidget Container Index))
  (Utilities|IsValid _widget
    (:Is%20Valid
      (Default|ResetSlot _widget))))

(event EventBeginPlay
  (Networking|SwitchHasAuthority
    (:Remote
      (bind _returnvalue (UserInterface|CreateWidget "/Game/_Main/Widgets/W_MainWidget.W_MainWidget_C" self))
      (bind _output_get (Variables|Default|SetMainWidgetRef _returnvalue))
      (UserInterface|Viewport|AddtoViewport _output_get 0))))

(event Input|KeyboardEvents|Tab
  (params (Key :type Key%20Structure :default "None"))
  (:Pressed
    (CallFunction|InventoryonClient)))

(event Input|KeyboardEvents|I
  (params (Key :type Key%20Structure :default "None"))
  (:Pressed
    (CallFunction|InventoryonClient)))

(fn ConstructionScript)

(fn GetInventoryWidget
  (params (Container :type E_ContainerType%20Enum :default "NewEnumerator0") (SlotIndex :type Integer))
  (return (Utilities|Array|Get(acopy) (Variables|/Game/_Main/Widgets/InventoryWidgets/W_ItemsContainerGrid.W_ItemsContainerGrid_C|GetSlots (Utilities|Select :Index Container :NewEnumerator0 (Variables|/Game/_Main/Widgets/InventoryWidgets/W_Inventory.W_Inventory_C|GetW_ItemsContainerGrid (Variables|/Game/_Main/Widgets/W_MainWidget.W_MainWidget_C|GetW_Inventory (Variables|Default|GetMainWidgetRef))) :NewEnumerator1 (Variables|/Game/_Main/Widgets/InventoryWidgets/W_Hotbar.W_Hotbar_C|GetW_ItemsContainerGrid (Variables|/Game/_Main/Widgets/W_MainWidget.W_MainWidget_C|GetW_Hotbar (Variables|Default|GetMainWidgetRef))) :NewEnumerator2 0 :NewEnumerator3 0)) SlotIndex)))

(fn GamePcRef
  (return self))